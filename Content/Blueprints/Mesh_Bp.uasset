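; Procedural mesh Blueprint that builds a flat grid of Nx by Ny vertices in its construction script.
; Nested loops use a math expression on each grid index, scaled by 100, to fill the position array.
; Those positions and generated grid triangles feed one procedural mesh section.
; The normals array receives the same values as positions rather than surface normals, and the event graph is empty.
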(event EventBeginPlay)

(event Collision|EventActorBeginOverlap
  (params (OtherActor :type Actor%20Object%20Reference)))

(event EventTick
  (params (DeltaSeconds :type Float%20%28single-precision%29)))

(fn ConstructionScript
  (bind _nx (LocalVariables|GetNx))
  (bind _ny (LocalVariables|GetNy))
  (bind _triangles (Class|KismetProceduralMeshLibrary|CreateGridMeshTriangles _nx _ny false))
  (for _index (range 0 (- _nx 1))
    (for _index_2 (range 0 (- _ny 1))
      (Utilities|Array|Add (LocalVariables|Getpositions) (* (|(Vector((i/({8D6678BA-0B43-C5E6-E596-C39F0065B8F7}-1)),(j/({B5A60D9D-D84B-BEE1-0991-0B8A8AE0B73E}-1)),0)) (Math|Conversions|ToFloat(Integer) _index) (Math|Conversions|ToFloat(Integer) _index_2)) 1e+02))
      (Utilities|Array|Add (LocalVariables|Getnormals) (* (|(Vector((i/({8D6678BA-0B43-C5E6-E596-C39F0065B8F7}-1)),(j/({B5A60D9D-D84B-BEE1-0991-0B8A8AE0B73E}-1)),0)) (Math|Conversions|ToFloat(Integer) _index) (Math|Conversions|ToFloat(Integer) _index_2)) 1e+02))))
  (Class|ProceduralMeshComponent|CreateMeshSectionLinearColor (Variables|Default|GetProceduralMesh) 0 (LocalVariables|Getpositions) _triangles (LocalVariables|Getnormals) 0 0 0 0 0 0 false))